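; Ether interactor component that links game actors such as terminals to the Ethereum manager for wallet, transfer and contract operations.
; Execute and BatchExecute forward requests to the supplied manager.
; BeginPlay polls until player states exist, then asks each to update bindings so server-side response handlers attach to their managers.
; Responses are routed by UserIndex to the matching player state, then re-broadcast to listeners on the owning client.
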(event `BatchExecute`
  (params (EtherManager :type "EtherManager Object Reference") (BatchRequestData :type "EtherlinkerBatchRequestData Structure"))
  ;[1 1 1] Process batch request
  (`/Engine/EditorBlueprintResources/StandardMacros.IsValid` EtherManager
    (:`Is Valid`
      (`EtherManager.ProcessBatchRequest` EtherManager BatchRequestData))))

(event `Execute`
  (params (EtherManager :type "EtherManager Object Reference") (OperationType :type "/Game/EtherlinkerExampleProject/Blueprints/Player/Global/BP_OperationTypes Enum" :default "NewEnumerator0") (RequestData :type "EtherlinkerRequestData Structure"))
  ;[1 1 1] Execute requested method
  (`/Engine/EditorBlueprintResources/StandardMacros.IsValid` EtherManager
    (:`Is Valid`
      (switch `/Game/EtherlinkerExampleProject/Blueprints/Player/Global/BP_OperationTypes` OperationType
        (:`NewEnumerator0`
          (`EtherManager.GetWalletBalance` EtherManager RequestData))
        (:`NewEnumerator1`
          (`EtherManager.ExecContractMethod` EtherManager RequestData))
        (:`NewEnumerator2`
          (`EtherManager.DeployContract` EtherManager RequestData))
        (:`NewEnumerator3`
          (`EtherManager.CreateWallet` EtherManager RequestData))
        (:`NewEnumerator5`
          (`EtherManager.TransferEther` EtherManager RequestData))))))

(event `OnBatchResponseReceived`
  (params (Result :type String) (Data :type "EtherlinkerBatchResponseData Structure"))
  (bind _playerarray (`GameStateBase.PlayerArray` (`GameplayStatics.GetGameState`)))
  ;[1 1 1] Call OnBatchResponseReceived for owning client
  (if (> (`KismetArrayLibrary.Array_Length` _playerarray) 0)
    (for _array_element _playerarray
      (bind _userindex (message `/Game/EtherlinkerExampleProject/Blueprints/Player/Global/BP_EtherManagerHolder.GetUserIndex` _array_element))
      (if (== _userindex (`KismetStringLibrary.Conv_StringToInt` (`.userIndex` (break `EtherlinkerBatchResponseData` Data))))
        (message `/Game/EtherlinkerExampleProject/Blueprints/Player/Global/BP_EtherManagerHolder.Execute On Batch Response Received` _array_element self Result Data)
        (break)))))

(event `OnResponseReceived`
  (params (Result :type String) (Data :type "EtherlinkerResponseData Structure"))
  (bind _playerarray (`GameStateBase.PlayerArray` (`GameplayStatics.GetGameState`)))
  ;[1 1 1] Call OnResponseReceived for owning client
  (if (> (`KismetArrayLibrary.Array_Length` _playerarray) 0)
    (for _array_element _playerarray
      (bind _userindex (message `/Game/EtherlinkerExampleProject/Blueprints/Player/Global/BP_EtherManagerHolder.GetUserIndex` _array_element))
      (if (== _userindex (`KismetStringLibrary.Conv_StringToInt` (`.userIndex` (break `EtherlinkerResponseData` Data))))
        (message `/Game/EtherlinkerExampleProject/Blueprints/Player/Global/BP_EtherManagerHolder.Execute On Response Received` _array_element self Result Data)
        (break)))))

(event `/Game/EtherlinkerExampleProject/Blueprints/Player/Global/BP_EtherInteractor.OnEtherResponseReceived`
  (params (Result :type String) (Data :type "EtherlinkerResponseData Structure"))
  ;[1 1 1] Dispatch Event To Listeners (such as BP_Terminal_01) on owning client
  (`self.OnResponseReceivedEvent` Result Data))

(event `/Game/EtherlinkerExampleProject/Blueprints/Player/Global/BP_EtherInteractor.OnEtherBatchResponseReceived`
  (params (Result :type String) (Data :type "EtherlinkerBatchResponseData Structure"))
  ;[1 1 1] Dispatch Batch Event To Listeners (such as BP_Terminal_01) on owning client
  (`self.OnBatchResponseReceivedEvent` Result Data))

(event `self.ReceiveBeginPlay`
  (bind _playerarray (`GameStateBase.PlayerArray` (`GameplayStatics.GetGameState`)))
  ;[1 1 1] Bind OnResponseReceived event on server side from client
  ;;[0.1812 0.1812 0.1812] From Local to Server on all Player States
  (if (> (`KismetArrayLibrary.Array_Length` _playerarray) 0) :!label _label
    (for _array_element _playerarray
      (message `/Game/EtherlinkerExampleProject/Blueprints/Player/Global/BP_EtherManagerHolder.Execute Update Bindings` _array_element self))
    (else
      (`KismetSystemLibrary.Delay` 0.1)
      (goto _label))))

(event `/Game/EtherlinkerExampleProject/Blueprints/Player/Global/BP_EtherInteractor.UpdateBindings`
  (bind _playerarray (`GameStateBase.PlayerArray` (`GameplayStatics.GetGameState`)))
  ;[1 1 1] Bind OnResponseReceived event on server side from client
  ;;[0.1812 0.1812 0.1812] On Server for all Player States
  (if (> (`KismetArrayLibrary.Array_Length` _playerarray) 0) :!label _label_2
    (for _array_element _playerarray
      (bind _ethermanager (message `/Game/EtherlinkerExampleProject/Blueprints/Player/Global/BP_EtherManagerHolder.GetEthereumManager` _array_element))
      (`/Engine/EditorBlueprintResources/StandardMacros.IsValid` _array_element
        (:`Is Valid`
          (add `EtherManager.OnResponseReceivedEvent` _ethermanager (delegate `OnResponseReceived`))
          (add `EtherManager.OnBatchResponseReceivedEvent` _ethermanager (delegate `OnBatchResponseReceived`)))))
    (else
      (`KismetSystemLibrary.Delay` 0.1)
      (goto _label_2))))