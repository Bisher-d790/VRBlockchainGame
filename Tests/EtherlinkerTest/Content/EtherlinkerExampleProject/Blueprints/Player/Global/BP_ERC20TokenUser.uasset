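; BP_ERC20TokenUser is an interface-style contract for a player's ERC20 token features in the Etherlinker example project, with no logic in its functions.
; It declares calls to initialize with a contract, buy tokens, check balance, query prices, and buy or check premium items and subscriptions.
; Each operation has an OnServerFromUI counterpart for menu-driven server requests.
; A getter and setter pair exposes the token user menu widget.
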(fn `BuyPremiumItem`
  (params (ItemId :type Integer))
  (returns (Result :type Boolean))
  (return false))

(fn `BuyPremiumItemOnServerFromUI`
  (params (ItemId :type Integer)))

(fn `BuyPremiumSubscription`
  (params (Days :type Integer) (SubscriptionTypeId :type Integer))
  (returns (Result :type Boolean))
  (return false))

(fn `BuyPremiumSubscriptionOnServerFromUI`
  (params (Days :type Integer) (SubscriptionTypeId :type Integer)))

(fn `BuyToken`
  (params (`ETH Amount` :type "Float (double-precision)"))
  (returns (Result :type Boolean))
  (return false))

(fn `BuyTokenOnServerFromUI`
  (params (`ETH Amount` :type "Float (double-precision)")))

(fn `CheckPremiumItem`
  (params (ItemId :type Integer))
  (returns (Result :type Boolean))
  (return false))

(fn `CheckPremiumItemOnServerFromUI`
  (params (ItemId :type Integer)))

(fn `CheckPremiumSubscription`
  (params (SubscriptionTypeId :type Integer))
  (returns (Result :type Boolean))
  (return false))

(fn `CheckPremiumSubscriptionOnServerFromUI`
  (params (SubscriptionTypeId :type Integer)))

(fn `CheckTokenBalance`
  (returns (Result :type Boolean))
  (return false))

(fn `CheckTokenBalanceOnServerFromUI`)

(fn `GetERC20TokenUserMenuWidget`
  (returns (ERC20TokenUserMenuWidget :type "UserWidget Object Reference"))
  (return null))

(fn `GetPremiumItemPrice`
  (params (ItemId :type Integer))
  (returns (Result :type Boolean))
  (return false))

(fn `GetPremiumItemPriceOnServerFromUI`
  (params (ItemId :type Integer)))

(fn `GetPremiumSubscriptionPricePerDay`
  (params (SubscriptionTypeId :type Integer))
  (returns (Result :type Boolean))
  (return false))

(fn `GetPremiumSubscriptionPricePerDayOnServerFromUI`
  (params (SubscriptionTypeId :type Integer)))

(fn `GetTokenPrice`
  (returns (Result :type Boolean))
  (return false))

(fn `GetTokenPriceOnServerFromUI`)

(fn `InitializeERC20TokenUser`
  (params (ContractAddress :type String) (ContractName :type String))
  (returns (Result :type Boolean))
  (return false))

(fn `InitializeERC20TokenUserOnServerFromUI`
  (params (ContractAddress :type String) (ContractName :type String)))

(fn `SetERC20TokenUserMenuWidget`
  (params (ERC20TokenUserMenuWidget :type "UserWidget Object Reference")))