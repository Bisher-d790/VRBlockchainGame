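; Interactive terminal prop that runs a configured Etherlinker Ethereum operation, such as wallet creation, balance query, contract call or deployment, or ETH transfer.
; Use checks wallet state, builds the request from its variables and player state, then executes it through BPEtherInteractorComponent, one call at a time.
; Responses matching its SenderId appear on the widget.
; Focus toggles a custom-depth highlight, while VR motion-controller overlap drives a timed progress bar for hold-to-use.
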(event `self.Use`
  (params (IsPlayer :type Boolean) (Interactor :type "Pawn Object Reference"))
  (bind _playerstate (`Pawn.PlayerState` Interactor))
  ;[1 1 1] Use event - Set variables and execute selected method
  (if (`self.CanBeUsed`)
    (bind _result (message `/Game/EtherlinkerExampleProject/Blueprints/Player/Global/BP_EtherManagerHolder.CheckWalletInitialization` _playerstate))
    (if (or _result (`|EnumEquality` (`self.OperationType`) "NewEnumerator3"))
      (bind _ethermanager (message `/Game/EtherlinkerExampleProject/Blueprints/Player/Global/BP_EtherManagerHolder.GetEthereumManager` _playerstate))
      (bind _userindex (message `/Game/EtherlinkerExampleProject/Blueprints/Player/Global/BP_EtherManagerHolder.GetUserIndex` _playerstate))
      (if (`self.CallCompleted`)
        (set `self.CallCompleted` false)
        (`GameplayStatics.PlaySound2D` "/Game/EtherlinkerExampleProject/Audio/Environment/Text_Pop_Cue.Text_Pop_Cue" 1.0 1.0 0.0 null null)
        (`KismetArrayLibrary.Array_Clear` (`self.ContractMethodParamTypesAsString`))
        (for _array_element (`self.ContractMethodParamTypes`)
          (`KismetArrayLibrary.Array_Add` (`self.ContractMethodParamTypesAsString`) (`|GetEnumeratorNameAsString` _array_element)))
        (`TextBlock.SetText` (`/Game/EtherlinkerExampleProject/Blueprints/UI/Widgets/BP_Terminal_UI.Terminal_Text` (cast `/Game/EtherlinkerExampleProject/Blueprints/UI/Widgets/BP_Terminal_UI` (`WidgetComponent.GetUserWidgetObject` (`self.Widget`)) :!pure true)) "Processing request...")
        ;;[1 1 1] Should we convert result from Wei to ETH?
        (if (`self.ShouldConvertResultFromWeiToEth`)
          (set `self.ConvertResultFromWeiToEth` "true")
          (else
            (set `self.ConvertResultFromWeiToEth` "false")))
        ;;[1 1 1] Should we use current wallet as default wallet address?
        (if (`self.UseCurrentWalletAsWalletAddress`)
          (bind _walletaddress (message `/Game/EtherlinkerExampleProject/Blueprints/Player/Global/BP_EtherManagerHolder.GetWalletAddress` _playerstate))
          (if (`KismetStringLibrary.NotEqual_StrStr` _walletaddress)
            (set `self.WalletAddress` _walletaddress)))
        ;;[1 1 1] Should we set current wallet address as a first parameter
        (if (`self.UseCurrentWalletAddressAsFirstParameter`)
          (bind _walletaddress_2 (message `/Game/EtherlinkerExampleProject/Blueprints/Player/Global/BP_EtherManagerHolder.GetWalletAddress` _playerstate))
          (if (`KismetStringLibrary.NotEqual_StrStr` _walletaddress_2)
            (`KismetArrayLibrary.Array_Set` (`self.ContractMethodParams`) 0 _walletaddress_2 true)))
        (`/Game/EtherlinkerExampleProject/Blueprints/Player/Global/BP_EtherInteractorComponent.Execute` (`self.BP_EtherInteractorComponent`) _ethermanager (`self.OperationType`) (make `EtherlinkerRequestData` (`self.SenderId`) (`KismetStringLibrary.Conv_IntToString` _userindex) (`self.ServerAddress`) (`self.WalletAddress`) (`self.ContractAddress`) (`self.ContractMethodName`) (`self.ContractName`) (`self.ContractMethodParams`) (`self.ContractMethodParamTypesAsString`) (`self.ConvertResultFromWeiToEth`) (`self.GasPrice`) (`self.GasLimit`) (`self.InfuraURL`) (`self.ReceiverAddress`) (`self.EthAmountToSend`) (`|GetEnumeratorNameAsString` (`self.OperationType`))))
        (else
          (`KismetSystemLibrary.PrintString` "Waiting for previous call completion" false)))
      (else
        (`TextBlock.SetText` (`/Game/EtherlinkerExampleProject/Blueprints/UI/Widgets/BP_Terminal_UI.Terminal_Text` (cast `/Game/EtherlinkerExampleProject/Blueprints/UI/Widgets/BP_Terminal_UI` (`WidgetComponent.GetUserWidgetObject` (`self.Widget`)) :!pure true)) "Error: Wallet is not initialized.")
        (`GameplayStatics.PlaySound2D` "/Game/EtherlinkerExampleProject/Audio/Environment/Text_Pop_Cue.Text_Pop_Cue" 1.0 1.0 0.0 null null)))))

(event `self.ReceiveBeginPlay`
  ;[1 1 1] On Response Received
  (add `/Game/EtherlinkerExampleProject/Blueprints/Player/Global/BP_EtherInteractorComponent.OnResponseReceivedEvent` (`self.BP_EtherInteractorComponent`) (delegate `OnEtherResponseReceived`)))

(event `OnEtherResponseReceived`
  (params (Result :type String) (Data :type "EtherlinkerResponseData Structure"))
  (bind (_senderid _userindex _data _operationtype) (break `EtherlinkerResponseData` Data))
  (bind (_lefts _rights) (`KismetStringLibrary.Split` _data ";"))
  (bind (_lefts_2 _rights_2) (`KismetStringLibrary.Split` _rights ";"))
  ;[1 1 1] On Response Received
  (if (`KismetStringLibrary.EqualEqual_StrStr` _senderid (`self.SenderId`))
    (set `self.CallCompleted` true)
    (if (`KismetStringLibrary.EqualEqual_StrStr` Result "success")
      (switch `string` _operationtype
        (:`getWalletBalance`
          (`TextBlock.SetText` (`/Game/EtherlinkerExampleProject/Blueprints/UI/Widgets/BP_Terminal_UI.Terminal_Text` (cast `/Game/EtherlinkerExampleProject/Blueprints/UI/Widgets/BP_Terminal_UI` (`WidgetComponent.GetUserWidgetObject` (`self.Widget`)) :!pure true)) (`KismetTextLibrary.Conv_StringToText` (`KismetStringLibrary.Concat_StrStr` "Wallet Balance: " _data))))
        (:`execContractMethod`
          (`TextBlock.SetText` (`/Game/EtherlinkerExampleProject/Blueprints/UI/Widgets/BP_Terminal_UI.Terminal_Text` (cast `/Game/EtherlinkerExampleProject/Blueprints/UI/Widgets/BP_Terminal_UI` (`WidgetComponent.GetUserWidgetObject` (`self.Widget`)) :!pure true)) (`KismetTextLibrary.Conv_StringToText` (`KismetStringLibrary.Concat_StrStr` "Contract Requested Value: " _data))))
        (:`deployContract`
          (`TextBlock.SetText` (`/Game/EtherlinkerExampleProject/Blueprints/UI/Widgets/BP_Terminal_UI.Terminal_Text` (cast `/Game/EtherlinkerExampleProject/Blueprints/UI/Widgets/BP_Terminal_UI` (`WidgetComponent.GetUserWidgetObject` (`self.Widget`)) :!pure true)) (`KismetTextLibrary.Conv_StringToText` (`KismetStringLibrary.Concat_StrStr` "Contract Address: " _data))))
        (:`createWallet`
          (`TextBlock.SetText` (`/Game/EtherlinkerExampleProject/Blueprints/UI/Widgets/BP_Terminal_UI.Terminal_Text` (cast `/Game/EtherlinkerExampleProject/Blueprints/UI/Widgets/BP_Terminal_UI` (`WidgetComponent.GetUserWidgetObject` (`self.Widget`)) :!pure true)) (`KismetTextLibrary.Conv_StringToText` (`KismetStringLibrary.Concat_StrStr` "Wallet Address: " (`.RightS` (`KismetStringLibrary.Split` _lefts ".")) " \nMnemonic: " _lefts_2 " \nPassword: " _rights_2))))
        (:`transferEther`
          (`TextBlock.SetText` (`/Game/EtherlinkerExampleProject/Blueprints/UI/Widgets/BP_Terminal_UI.Terminal_Text` (cast `/Game/EtherlinkerExampleProject/Blueprints/UI/Widgets/BP_Terminal_UI` (`WidgetComponent.GetUserWidgetObject` (`self.Widget`)) :!pure true)) (`KismetTextLibrary.Conv_StringToText` (`KismetStringLibrary.Concat_StrStr` "ETH transfer result: " _data)))))
      (else
        (`TextBlock.SetText` (`/Game/EtherlinkerExampleProject/Blueprints/UI/Widgets/BP_Terminal_UI.Terminal_Text` (cast `/Game/EtherlinkerExampleProject/Blueprints/UI/Widgets/BP_Terminal_UI` (`WidgetComponent.GetUserWidgetObject` (`self.Widget`)) :!pure true)) (`KismetTextLibrary.Conv_StringToText` _data))))))

(event `self.StartFocus`
  ;[1 1 1] Focus glow
  (`PrimitiveComponent.SetCustomDepthStencilValue` (`self.Terminal`) 252)
  (`PrimitiveComponent.SetRenderCustomDepth` (`self.Terminal`) true))

(event `self.Box.OnComponentBeginOverlap`
  (params (OverlappedComponent :type "PrimitiveComponent Object Reference") (OtherActor :type "Actor Object Reference") (OtherComp :type "PrimitiveComponent Object Reference") (OtherBodyIndex :type Integer) (bFromSweep :type Boolean) (SweepResult :type "HitResult Structure (by ref)"))
  ;[1 1 1] VR Use
  (bind _asbp_motion_controller (cast `/Game/EtherlinkerExampleProject/Blueprints/Player/VR/BP_MotionController` OtherActor))
  (`/Engine/EditorBlueprintResources/StandardMacros.IsValid` (`self.OverlappedMotionController`)
    (:`Is Not Valid`
      (set `self.IsOverlappedByMotionController` true)
      (set `self.OverlappedMotionController` _asbp_motion_controller)
      (set `self.CurrentOverlappingTime` 0.0)
      (if (`KismetSystemLibrary.K2_TimerExistsHandle` (`self.OverlappingTimerHandle`))
        (`KismetSystemLibrary.K2_UnPauseTimerHandle` (`self.OverlappingTimerHandle`))
        (else
          (bind _returnvalue (`KismetSystemLibrary.K2_SetTimerDelegate` (delegate `UpdateOverlappingTime`) 0.1 true))
          (set `self.OverlappingTimerHandle` _returnvalue))))))

(event `self.StopFocus`
  ;[1 1 1] Focus glow
  (`PrimitiveComponent.SetRenderCustomDepth` (`self.Terminal`) false))

(event `UpdateOverlappingTime`
  ;[1 1 1] VR Use
  (set `self.CurrentOverlappingTime` (+ (`self.CurrentOverlappingTime`) 1.0)))

(event `self.Box.OnComponentEndOverlap`
  (params (OverlappedComponent :type "PrimitiveComponent Object Reference") (OtherActor :type "Actor Object Reference") (OtherComp :type "PrimitiveComponent Object Reference") (OtherBodyIndex :type Integer))
  (bind _overlappingtimerhandle (`self.OverlappingTimerHandle`))
  ;[1 1 1] VR Use
  (bind _asbp_motion_controller (cast `/Game/EtherlinkerExampleProject/Blueprints/Player/VR/BP_MotionController` OtherActor))
  (if (== _asbp_motion_controller (`self.OverlappedMotionController`))
    (set `self.IsOverlappedByMotionController` false)
    (set `self.OverlappedMotionController` null)
    (if (`KismetSystemLibrary.K2_TimerExistsHandle` _overlappingtimerhandle)
      (`KismetSystemLibrary.K2_PauseTimerHandle` _overlappingtimerhandle)
      (`|ExecutionSequence`
        (:`then_0`
          (bind _returnvalue (`Image.GetDynamicMaterial` (`/Game/EtherlinkerExampleProject/Blueprints/UI/Widgets/BP_Terminal_UI.ProgressBar` (cast `/Game/EtherlinkerExampleProject/Blueprints/UI/Widgets/BP_Terminal_UI` (`WidgetComponent.GetUserWidgetObject` (`self.Widget`)) :!pure true)) :!label _label))
          (`MaterialInstanceDynamic.SetScalarParameterValue` _returnvalue "Alpha" 0.0))
        (:`then_1`
          (goto _label_2 :!via `Reset`))))))

(event `self.ReceiveTick`
  (params (DeltaSeconds :type "Float (single-precision)"))
  ;[1 1 1] VR Use
  (`/Engine/EditorBlueprintResources/StandardMacros.IsValid` (`self.OverlappedMotionController`)
    (:`Is Valid`
      (if (`self.IsOverlappedByMotionController`)
        (if (>= (`self.CurrentOverlappingTime`) (`self.RequiredOverlappingTime`))
          (`/Engine/EditorBlueprintResources/StandardMacros.DoOnce` false :!label _label_2
            (:`Completed`
              (`self.Use` true (`/Game/EtherlinkerExampleProject/Blueprints/Player/VR/BP_MotionController.ParentPawn` (`self.OverlappedMotionController`)))
              (goto _label)))
          (else
            (bind _returnvalue (`Image.GetDynamicMaterial` (`/Game/EtherlinkerExampleProject/Blueprints/UI/Widgets/BP_Terminal_UI.ProgressBar` (cast `/Game/EtherlinkerExampleProject/Blueprints/UI/Widgets/BP_Terminal_UI` (`WidgetComponent.GetUserWidgetObject` (`self.Widget`)) :!pure true))))
            (`MaterialInstanceDynamic.SetScalarParameterValue` _returnvalue "Alpha" (/ (`self.CurrentOverlappingTime`) (`self.RequiredOverlappingTime`)))))))))

(fn `GetStaticMeshComponent`
  (returns (StaticMesh :type "StaticMeshComponent Object Reference"))
  (return null))

(fn `UserConstructionScript`)