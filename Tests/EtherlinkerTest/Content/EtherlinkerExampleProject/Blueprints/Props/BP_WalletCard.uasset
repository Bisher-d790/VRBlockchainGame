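; BP_WalletCard is a grabbable wallet card prop for motion controllers that displays a wallet address.
; SetWalletCardAddress writes the address into the terminal text of two BP_WalletCardAddress_UI widgets on the card.
; Pickup disables physics and snaps the card to WalletCardSocket on MannequinHand or HandMesh, depending on the controller's IsHandCollisionActive flag.
; Drop re-enables physics and detaches the card, keeping its world transform.
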(event `SetWalletCardAddress`
  (params (WalletAddress :type String))
  (bind _returnvalue (`KismetTextLibrary.Conv_StringToText` WalletAddress))
  (`TextBlock.SetText` (`/Game/EtherlinkerExampleProject/Blueprints/UI/Widgets/BP_WalletCardAddress_UI.Terminal_Text` (cast `/Game/EtherlinkerExampleProject/Blueprints/UI/Widgets/BP_WalletCardAddress_UI` (`WidgetComponent.GetUserWidgetObject` (`self.Widget`)) :!pure true)) _returnvalue)
  (`TextBlock.SetText` (`/Game/EtherlinkerExampleProject/Blueprints/UI/Widgets/BP_WalletCardAddress_UI.Terminal_Text` (cast `/Game/EtherlinkerExampleProject/Blueprints/UI/Widgets/BP_WalletCardAddress_UI` (`WidgetComponent.GetUserWidgetObject` (`self.Widget1`)) :!pure true)) _returnvalue))

(event `/Game/EtherlinkerExampleProject/Blueprints/Player/VR/PickupActorInterface.Pickup`
  (params (AttachTo :type "Actor Object Reference"))
  (bind _returnvalue (`self.K2_GetRootComponent`))
  (bind _asbp_motion_controller (cast `/Game/EtherlinkerExampleProject/Blueprints/Player/VR/BP_MotionController` AttachTo :!pure true))
  (`PrimitiveComponent.SetSimulatePhysics` (`self.StaticMeshComponent`) false)
  (if (`/Game/EtherlinkerExampleProject/Blueprints/Player/VR/BP_MotionController.IsHandCollisionActive` _asbp_motion_controller)
    (`SceneComponent.K2_AttachToComponent` _returnvalue (`/Game/EtherlinkerExampleProject/Blueprints/Player/VR/BP_MotionController.MannequinHand` _asbp_motion_controller) "WalletCardSocket" "SnapToTarget" "SnapToTarget" "KeepWorld" false)
    (else
      (`SceneComponent.K2_AttachToComponent` _returnvalue (`/Game/EtherlinkerExampleProject/Blueprints/Player/VR/BP_MotionController.HandMesh` _asbp_motion_controller) "WalletCardSocket" "SnapToTarget" "SnapToTarget" "KeepWorld" false))))

(event `/Game/EtherlinkerExampleProject/Blueprints/Player/VR/PickupActorInterface.Drop`
  (`PrimitiveComponent.SetSimulatePhysics` (`self.StaticMeshComponent`) true)
  (`self.K2_DetachFromActor` "KeepWorld" "KeepWorld" "KeepWorld"))

(fn `UserConstructionScript`)