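; Portable terminal prop that a motion controller can pick up and drop.
; Pickup turns off physics on the Terminal and attaches the root to the controller, keeping world transform.
; The attach target is MannequinHand when the controller's hand collision is active, otherwise the WalletCardSocket on HandMesh.
; Drop re-enables physics and detaches the actor in place.
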(event `/Game/EtherlinkerExampleProject/Blueprints/Player/VR/PickupActorInterface.Pickup`
  (params (AttachTo :type "Actor Object Reference"))
  (bind _returnvalue (`self.K2_GetRootComponent`))
  (bind _asbp_motion_controller (cast `/Game/EtherlinkerExampleProject/Blueprints/Player/VR/BP_MotionController` AttachTo :!pure true))
  (`PrimitiveComponent.SetSimulatePhysics` (`self.Terminal`) false)
  (if (`/Game/EtherlinkerExampleProject/Blueprints/Player/VR/BP_MotionController.IsHandCollisionActive` _asbp_motion_controller)
    (`SceneComponent.K2_AttachToComponent` _returnvalue (`/Game/EtherlinkerExampleProject/Blueprints/Player/VR/BP_MotionController.MannequinHand` _asbp_motion_controller) "None" "KeepWorld" "KeepWorld" "KeepWorld" false)
    (else
      (`SceneComponent.K2_AttachToComponent` _returnvalue (`/Game/EtherlinkerExampleProject/Blueprints/Player/VR/BP_MotionController.HandMesh` _asbp_motion_controller) "WalletCardSocket" "KeepWorld" "KeepWorld" "KeepWorld" false))))

(event `/Game/EtherlinkerExampleProject/Blueprints/Player/VR/PickupActorInterface.Drop`
  (`PrimitiveComponent.SetSimulatePhysics` (`self.Terminal`) true)
  (`self.K2_DetachFromActor` "KeepWorld" "KeepWorld" "KeepWorld"))

(fn `UserConstructionScript`
  (`parent.UserConstructionScript`))