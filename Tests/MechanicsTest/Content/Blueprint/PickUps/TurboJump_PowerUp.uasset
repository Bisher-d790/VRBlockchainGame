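; Turbo jump power-up pickup that temporarily boosts the jump height of the actor that activates it.
; On activation it stores that actor and sets its CharacterMovementComponent JumpZVelocity to NormalJump multiplied by TurboFactor.
; On expiry it resets the stored actor to the preset NormalJump value, rather than a captured original, then calls the parent's expiry logic.
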(event `self.OnActivated`
  (params (ForActor :type "Actor Object Reference"))
  (bind _returnvalue (`self.GetComponentByClass` ForActor "/Script/Engine.CharacterMovementComponent"))
  (set `self.TargetPlayer` ForActor)
  (`/Engine/EditorBlueprintResources/StandardMacros.IsValid` _returnvalue
    (:`Is Valid`
      (set `CharacterMovementComponent.JumpZVelocity` (* (`self.TurboFactor`) (`self.NormalJump`)) _returnvalue))))

(event `self.OnExpired`
  (bind _returnvalue (`self.GetComponentByClass` (`self.TargetPlayer`) "/Script/Engine.CharacterMovementComponent"))
  (`/Engine/EditorBlueprintResources/StandardMacros.IsValid` _returnvalue
    (:`Is Valid`
      (set `CharacterMovementComponent.JumpZVelocity` (`self.NormalJump`) _returnvalue))
    (:`Is Not Valid`
      _))
  (`parent.OnExpired`))

(fn `UserConstructionScript`
  (`parent.UserConstructionScript`))