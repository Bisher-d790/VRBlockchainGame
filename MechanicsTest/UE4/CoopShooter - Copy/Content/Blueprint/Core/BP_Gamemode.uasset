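; Game mode Blueprint that handles tracker bot spawning, kill scoring and the game-over switch to spectators.
; SpawnBot runs an EQS spawn-location query, then spawns a BP_TrackerBot with a debug sphere at each returned location.
; An actor-killed binding awards score to the killer's SPlayerState only when a player kills a non-player pawn.
; GameOverLogic spawns a spectator per player and has that player's controller possess it.
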(event `self.SpawnBot`
  (bind _returnvalue (`EnvQueryManager.RunEQSQuery` "/Game/Blueprint/AI/EQS_FindSpawnLocation.EQS_FindSpawnLocation" self "RandomBest25Pct"))
  (add `EnvQueryInstanceBlueprintWrapper.OnQueryFinishedEvent` _returnvalue (delegate `OnQueryFinishedEvent_Event`)))

(event `OnQueryFinishedEvent_Event`
  (params (QueryInstance :type "EnvQueryInstanceBlueprintWrapper Object Reference") (QueryStatus :type "EEnvQueryStatus Enum" :default "Processing"))
  (bind (_resultlocations _returnvalue) (`EnvQueryInstanceBlueprintWrapper.GetQueryResultsAsLocations` QueryInstance))
  (if _returnvalue
    (for _array_element _resultlocations
      (`KismetSystemLibrary.DrawDebugSphere` _array_element 100.0 12 (struct :`R` 1.0 :`G` 0.422123 :`A` 1.0) 2.0 5.0)
      (`|SpawnActorFromClass` "/Game/Blueprint/AI/BP_TrackerBot.BP_TrackerBot_C" (`KismetMathLibrary.Conv_VectorToTransform` _array_element) "AdjustIfPossibleButDontSpawnIfColliding" "OverrideRootScale" null null))))

(event `self.ReceiveBeginPlay`
  (add `self.OnActorKilled` (delegate `OnActorKilled_Event`)))

(event `OnActorKilled_Event` :!signature `self.OnActorKilled`
  (params (VictimActor :type "Actor Object Reference") (KillerActor :type "Actor Object Reference") (KillerController :type "Controller Object Reference"))
  ;[1 1 1] Prevent scoring from killing other player
  (bind _aspawn (cast `Pawn` VictimActor))
  (if (`Pawn.IsPlayerControlled` _aspawn)
    _
    (elif (`Controller.IsPlayerController` KillerController)
      (bind _assplayer_state (cast `SPlayerState` (`Pawn.PlayerState` (`Controller.K2_GetPawn` KillerController))))
      (`SPlayerState.AddScore` _assplayer_state (`self.KillScore`))
      (`KismetSystemLibrary.PrintString` (`KismetStringLibrary.Conv_DoubleToString` (`PlayerState.Score` _assplayer_state)) true true (struct :`R` 0.007164 :`G` 0.5625 :`A` 1.0)))))

(fn `GameOver_Logic`
  (locals (SpawnTransform :type "Transform Structure" :default "-6682.809570,6841.060547,7633.479492|-14.062491,-39.374931,0.000000|1.000000,1.000000,1.000000"))
  (bind _returnvalue (`self.GetNumPlayers`))
  (for _index (range (+ _returnvalue 1))
    (bind _returnvalue_2 (`GameplayStatics.GetPlayerController` _index))
    (bind _returnvalue_3 (`|SpawnActorFromClass` (`self.SpectatorClass`) (`local.SpawnTransform`) "AlwaysSpawn" "OverrideRootScale" _returnvalue_2 (`GameplayStatics.GetPlayerPawn` _index)))
    (`Controller.Possess` _returnvalue_2 _returnvalue_3)))

(fn `UserConstructionScript`)