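; Game mode Blueprint that handles kill scoring and switches players to spectators on game over.
; On BeginPlay it binds to OnActorKilled, awarding the kill score to the killing player's SPlayerState only when the victim is a non-player pawn.
; Each award prints the score on screen.
; GameOverLogic loops over player indices, spawning a spectator for each and having that player's controller possess it.
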(event `self.ReceiveBeginPlay`
  (add `self.OnActorKilled` (delegate `OnActorKilled_Event`)))

(event `OnActorKilled_Event` :!signature `self.OnActorKilled`
  (params (VictimActor :type "Actor Object Reference") (KillerActor :type "Actor Object Reference") (KillerController :type "Controller Object Reference"))
  ;[1 1 1] Prevent scoring from killing other player
  (bind _aspawn (cast `Pawn` VictimActor))
  (if (`Pawn.IsPlayerControlled` _aspawn)
    _
    (elif (`Controller.IsPlayerController` KillerController)
      (bind _assplayer_state (cast `SPlayerState` (`Pawn.PlayerState` (`Controller.K2_GetPawn` KillerController))))
      (`SPlayerState.AddScore` _assplayer_state (`self.KillScore`))
      (`KismetSystemLibrary.PrintString` (`KismetStringLibrary.Conv_DoubleToString` (`PlayerState.Score` _assplayer_state)) true true (struct :`R` 0.007164 :`G` 0.5625 :`A` 1.0)))))

(fn `GameOver_Logic`
  (locals (SpawnTransform :type "Transform Structure" :default "-6682.809570,6841.060547,7633.479492|-14.062491,-39.374866,0.000000|1.000000,1.000000,1.000000"))
  (bind _returnvalue (`self.GetNumPlayers`))
  (for _index (range (+ _returnvalue 1))
    (bind _returnvalue_2 (`GameplayStatics.GetPlayerController` _index))
    (bind _returnvalue_3 (`|SpawnActorFromClass` (`self.SpectatorClass`) (`local.SpawnTransform`) "AlwaysSpawn" "OverrideRootScale" _returnvalue_2 (`GameplayStatics.GetPlayerPawn` _index)))
    (`Controller.Possess` _returnvalue_2 _returnvalue_3)))

(fn `UserConstructionScript`)