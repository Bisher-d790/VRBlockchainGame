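; Speed boost power-up that temporarily raises the walk speed of the actor that activates it.
; On activation it stores that actor and sets its CharacterMovementComponent's MaxWalkSpeed to NormalSpeed times SuperSpeedFactor.
; On expiry it resets the speed to the configured NormalSpeed rather than a saved original, then calls the parent's expiry logic.
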(event `self.OnActivated`
  (params (ForActor :type "Actor Object Reference"))
  (bind _output_get (set `self.TargetPlayer` ForActor))
  (bind _returnvalue (`self.GetComponentByClass` _output_get "/Script/Engine.CharacterMovementComponent"))
  (`/Engine/EditorBlueprintResources/StandardMacros.IsValid` _returnvalue
    (:`Is Valid`
      (set `CharacterMovementComponent.MaxWalkSpeed` (* (`self.SuperSpeedFactor`) (`self.NormalSpeed`)) _returnvalue))))

(event `self.OnExpired`
  (bind _returnvalue (`self.GetComponentByClass` (`self.TargetPlayer`) "/Script/Engine.CharacterMovementComponent"))
  (`/Engine/EditorBlueprintResources/StandardMacros.IsValid` _returnvalue
    (:`Is Valid`
      (set `CharacterMovementComponent.MaxWalkSpeed` (`self.NormalSpeed`) _returnvalue))
    (:`Is Not Valid`
      _))
  (`parent.OnExpired`))

(fn `UserConstructionScript`)