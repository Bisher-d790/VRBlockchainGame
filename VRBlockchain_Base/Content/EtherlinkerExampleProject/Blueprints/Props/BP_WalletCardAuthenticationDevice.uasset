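; VR terminal prop that stores wallet data to, or initializes it from, a wallet card placed on it.
; A card collision box registers physics-simulating cards, while holding a motion controller in the store or load box picks the mode and fills a timed progress bar.
; A full bar fires once per hold, sending the request to the server through PlayerState.
; Update events write encrypted data to the card and show results on the terminal widget.
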(event `UseAuthenticationDevice`
  (bind _walletcard (`self.WalletCard`))
  (bind _playerstate (`Controller.PlayerState` (`GameplayStatics.GetPlayerController` 0)))
  ;[1 1 1] Use Authentication Device
  (`/Engine/EditorBlueprintResources/StandardMacros.IsValid` (`self.WalletCard`)
    (:`Is Valid`
      (if (`self.IsCardPlaced`)
        (if (`self.IsStoringData`)
          (message `/Game/EtherlinkerExampleProject/Blueprints/Player/Global/BP_EtherManagerHolder.StoreWalletDataToWalletCardOnServer` _playerstate self)
          (else
            (message `/Game/EtherlinkerExampleProject/Blueprints/Player/Global/BP_EtherManagerHolder.InitializeWalletDataFromWalletCardOnServer` _playerstate (`/Game/EtherlinkerExampleProject/Blueprints/Props/BP_WalletCard.IsWalletDataStored` _walletcard) (`/Game/EtherlinkerExampleProject/Blueprints/Props/BP_WalletCard.EncryptedWalletAddress` _walletcard) (`/Game/EtherlinkerExampleProject/Blueprints/Props/BP_WalletCard.EncryptedWalletPassword` _walletcard) (`/Game/EtherlinkerExampleProject/Blueprints/Props/BP_WalletCard.EncryptedWalletMnemonic` _walletcard) (`/Game/EtherlinkerExampleProject/Blueprints/Props/BP_WalletCard.EncryptedWalletPath` _walletcard) (`/Game/EtherlinkerExampleProject/Blueprints/Props/BP_WalletCard.EncryptedWalletAuthType` _walletcard) self)))
        (else
          (`self.UpdateCardInfo` "Error: Wallet Card is not placed" :!label _label)
          (`GameplayStatics.PlaySound2D` "/Game/EtherlinkerExampleProject/Audio/Environment/Text_Pop_Cue.Text_Pop_Cue" 1.0 1.0 0.0 null null))))
    (:`Is Not Valid`
      (goto _label))))

(event `self.StoreDataCollisionBox.OnComponentBeginOverlap`
  (params (OverlappedComponent :type "PrimitiveComponent Object Reference") (OtherActor :type "Actor Object Reference") (OtherComp :type "PrimitiveComponent Object Reference") (OtherBodyIndex :type Integer) (bFromSweep :type Boolean) (SweepResult :type "HitResult Structure (by ref)"))
  ;[1 1 1] Store Data Collision
  (bind _asbp_motion_controller (cast `/Game/EtherlinkerExampleProject/Blueprints/Player/VR/BP_MotionController` OtherActor))
  (cast `SphereComponent` OtherComp)
  (`/Engine/EditorBlueprintResources/StandardMacros.IsValid` (`self.OverlappedMotionController`)
    (:`Is Not Valid`
      (set `self.IsOverlappedByMotionController` true)
      (set `self.OverlappedMotionController` _asbp_motion_controller)
      (set `self.CurrentOverlappingTime` 0.0)
      (set `self.IsStoringData` true)
      (if (`KismetSystemLibrary.K2_TimerExistsHandle` (`self.OverlappingTimerHandle`))
        (`KismetSystemLibrary.K2_UnPauseTimerHandle` (`self.OverlappingTimerHandle`))
        (else
          (bind _returnvalue (`KismetSystemLibrary.K2_SetTimerDelegate` (delegate `UpdateOverlappingTime`) 0.1 true))
          (set `self.OverlappingTimerHandle` _returnvalue))))))

(event `self.StoreDataCollisionBox.OnComponentEndOverlap`
  (params (OverlappedComponent :type "PrimitiveComponent Object Reference") (OtherActor :type "Actor Object Reference") (OtherComp :type "PrimitiveComponent Object Reference") (OtherBodyIndex :type Integer))
  (bind _overlappingtimerhandle (`self.OverlappingTimerHandle`))
  ;[1 1 1] Store Data Collision
  (bind _asbp_motion_controller (cast `/Game/EtherlinkerExampleProject/Blueprints/Player/VR/BP_MotionController` OtherActor))
  (cast `SphereComponent` OtherComp)
  (if (== _asbp_motion_controller (`self.OverlappedMotionController`))
    (set `self.IsOverlappedByMotionController` false)
    (set `self.OverlappedMotionController` null)
    (if (`KismetSystemLibrary.K2_TimerExistsHandle` _overlappingtimerhandle)
      (`KismetSystemLibrary.K2_PauseTimerHandle` _overlappingtimerhandle)
      (`|ExecutionSequence`
        (:`then_0`
          ;[1 1 1] Event Tick
          (bind _returnvalue (`Image.GetDynamicMaterial` (`/Game/EtherlinkerExampleProject/Blueprints/UI/Widgets/BP_Terminal_UI.ProgressBar` (cast `/Game/EtherlinkerExampleProject/Blueprints/UI/Widgets/BP_Terminal_UI` (`WidgetComponent.GetUserWidgetObject` (`self.Widget`)) :!pure true)) :!label _label_2))
          (`MaterialInstanceDynamic.SetScalarParameterValue` _returnvalue "Alpha" 0.0))
        (:`then_1`
          (goto _label_3 :!via `Reset`))))))

(event `UpdateOverlappingTime`
  ;[1 1 1] Store Data Collision
  (set `self.CurrentOverlappingTime` (+ (`self.CurrentOverlappingTime`) 1.0)))

(event `self.ReceiveTick`
  (params (DeltaSeconds :type "Float (single-precision)"))
  ;[1 1 1] Event Tick
  (`/Engine/EditorBlueprintResources/StandardMacros.IsValid` (`self.OverlappedMotionController`)
    (:`Is Valid`
      (if (`self.IsOverlappedByMotionController`)
        (if (>= (`self.CurrentOverlappingTime`) (`self.RequiredOverlappingTime`))
          (`/Engine/EditorBlueprintResources/StandardMacros.DoOnce` false :!label _label_3
            (:`Completed`
              (`self.UseAuthenticationDevice`)
              (goto _label_2)))
          (else
            (bind _returnvalue (`Image.GetDynamicMaterial` (`/Game/EtherlinkerExampleProject/Blueprints/UI/Widgets/BP_Terminal_UI.ProgressBar` (cast `/Game/EtherlinkerExampleProject/Blueprints/UI/Widgets/BP_Terminal_UI` (`WidgetComponent.GetUserWidgetObject` (`self.Widget`)) :!pure true))))
            (`MaterialInstanceDynamic.SetScalarParameterValue` _returnvalue "Alpha" (/ (`self.CurrentOverlappingTime`) (`self.RequiredOverlappingTime`)))))))))

(event `self.LoadDataCollisionBox.OnComponentBeginOverlap`
  (params (OverlappedComponent :type "PrimitiveComponent Object Reference") (OtherActor :type "Actor Object Reference") (OtherComp :type "PrimitiveComponent Object Reference") (OtherBodyIndex :type Integer) (bFromSweep :type Boolean) (SweepResult :type "HitResult Structure (by ref)"))
  ;[1 1 1] Load Data Collision
  (bind _asbp_motion_controller (cast `/Game/EtherlinkerExampleProject/Blueprints/Player/VR/BP_MotionController` OtherActor))
  (cast `SphereComponent` OtherComp)
  (`/Engine/EditorBlueprintResources/StandardMacros.IsValid` (`self.OverlappedMotionController`)
    (:`Is Not Valid`
      (set `self.IsOverlappedByMotionController` true)
      (set `self.OverlappedMotionController` _asbp_motion_controller)
      (set `self.CurrentOverlappingTime` 0.0)
      (set `self.IsStoringData` false)
      (if (`KismetSystemLibrary.K2_TimerExistsHandle` (`self.OverlappingTimerHandle`))
        (`KismetSystemLibrary.K2_UnPauseTimerHandle` (`self.OverlappingTimerHandle`))
        (else
          (bind _returnvalue (`KismetSystemLibrary.K2_SetTimerDelegate` (delegate `UpdateOverlappingTime`) 0.1 true))
          (set `self.OverlappingTimerHandle` _returnvalue))))))

(event `self.LoadDataCollisionBox.OnComponentEndOverlap`
  (params (OverlappedComponent :type "PrimitiveComponent Object Reference") (OtherActor :type "Actor Object Reference") (OtherComp :type "PrimitiveComponent Object Reference") (OtherBodyIndex :type Integer))
  (bind _overlappingtimerhandle (`self.OverlappingTimerHandle`))
  ;[1 1 1] Load Data Collision
  (bind _asbp_motion_controller (cast `/Game/EtherlinkerExampleProject/Blueprints/Player/VR/BP_MotionController` OtherActor))
  (cast `SphereComponent` OtherComp)
  (if (== _asbp_motion_controller (`self.OverlappedMotionController`))
    (set `self.IsOverlappedByMotionController` false)
    (set `self.OverlappedMotionController` null)
    (if (`KismetSystemLibrary.K2_TimerExistsHandle` _overlappingtimerhandle)
      (`KismetSystemLibrary.K2_PauseTimerHandle` _overlappingtimerhandle)
      (`|ExecutionSequence`
        (:`then_0`
          (goto _label_2))
        (:`then_1`
          (goto _label_3 :!via `Reset`))))))

(event `self.UpdateWalletCardData`
  (params (EncryptedWalletAddress :type String) (EncryptedWalletPassword :type String) (EncryptedWalletMnemonic :type String) (EncryptedWalletPath :type String) (EncryptedWalletAuthType :type String) (IsWalletDataStored :type Boolean))
  (bind _walletcard (`self.WalletCard`))
  ;[1 1 1] Update Wallet Card Data
  (set `/Game/EtherlinkerExampleProject/Blueprints/Props/BP_WalletCard.EncryptedWalletAddress` EncryptedWalletAddress _walletcard)
  (set `/Game/EtherlinkerExampleProject/Blueprints/Props/BP_WalletCard.EncryptedWalletPassword` EncryptedWalletPassword _walletcard)
  (set `/Game/EtherlinkerExampleProject/Blueprints/Props/BP_WalletCard.EncryptedWalletMnemonic` EncryptedWalletMnemonic _walletcard)
  (set `/Game/EtherlinkerExampleProject/Blueprints/Props/BP_WalletCard.EncryptedWalletPath` EncryptedWalletPath _walletcard)
  (set `/Game/EtherlinkerExampleProject/Blueprints/Props/BP_WalletCard.EncryptedWalletAuthType` EncryptedWalletAuthType _walletcard)
  (set `/Game/EtherlinkerExampleProject/Blueprints/Props/BP_WalletCard.IsWalletDataStored` IsWalletDataStored _walletcard))

(event `self.UpdateCardInfo`
  (params (Result :type String) (WalletAddress :type String))
  ;[1 1 1] Update Card Info
  (if (`KismetStringLibrary.NotEqual_StrStr` WalletAddress "")
    (`/Game/EtherlinkerExampleProject/Blueprints/Props/BP_WalletCard.SetWalletCardAddress` (`self.WalletCard`) WalletAddress))
  (`TextBlock.SetText` (`/Game/EtherlinkerExampleProject/Blueprints/UI/Widgets/BP_Terminal_UI.Terminal_Text` (cast `/Game/EtherlinkerExampleProject/Blueprints/UI/Widgets/BP_Terminal_UI` (`WidgetComponent.GetUserWidgetObject` (`self.Widget`)) :!pure true)) (`KismetTextLibrary.Conv_StringToText` Result))
  (`GameplayStatics.PlaySound2D` "/Game/EtherlinkerExampleProject/Audio/Environment/Text_Pop_Cue.Text_Pop_Cue" 1.0 1.0 0.0 null null))

(event `self.WalletCardCollisionBox.OnComponentBeginOverlap`
  (params (OverlappedComponent :type "PrimitiveComponent Object Reference") (OtherActor :type "Actor Object Reference") (OtherComp :type "PrimitiveComponent Object Reference") (OtherBodyIndex :type Integer) (bFromSweep :type Boolean) (SweepResult :type "HitResult Structure (by ref)"))
  ;[1 1 1] Check if wallet card was placed
  (bind _asbp_wallet_card (cast `/Game/EtherlinkerExampleProject/Blueprints/Props/BP_WalletCard` OtherActor))
  (if (`SceneComponent.IsSimulatingPhysics` (`StaticMeshActor.StaticMeshComponent` _asbp_wallet_card) "None")
    (set `self.IsCardPlaced` true)
    (set `self.WalletCard` _asbp_wallet_card)))

(event `self.WalletCardCollisionBox.OnComponentEndOverlap`
  (params (OverlappedComponent :type "PrimitiveComponent Object Reference") (OtherActor :type "Actor Object Reference") (OtherComp :type "PrimitiveComponent Object Reference") (OtherBodyIndex :type Integer))
  ;[1 1 1] Check if wallet card was placed
  (bind _asbp_wallet_card (cast `/Game/EtherlinkerExampleProject/Blueprints/Props/BP_WalletCard` OtherActor))
  (if (== _asbp_wallet_card (`self.WalletCard`))
    (set `self.IsCardPlaced` false)
    (set `self.WalletCard` null)))

(fn `GenerateRandomEncryptionKey`
  (returns (EncryptionKey :type String))
  (return (`KismetStringLibrary.Concat_StrStr` (`KismetStringLibrary.Conv_DoubleToString` (`KismetMathLibrary.RandomFloat`)) (`KismetStringLibrary.Conv_DoubleToString` (`KismetMathLibrary.RandomFloat`)) (`KismetStringLibrary.Conv_DoubleToString` (`KismetMathLibrary.RandomFloat`)))))

(fn `OnRep_CurrentOverlappingTime`)

(fn `UserConstructionScript`)