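; BP_VROnlyBlockingVolume is a trigger Blueprint that blocks off an area for players not in VR mode.
; On BeginPlay, if IsActive, it asks the first player controller via CheckVRModeMessage whether VR mode is on.
; When it is not, it reveals the Cube and Widget and sets both the Cube and BlockingVolume to the BlockAllDynamic collision profile.
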(event `self.ReceiveBeginPlay`
  (bind _cube (`self.Cube`))
  (if (`self.IsActive`)
    (bind _result (message `/Game/EtherlinkerExampleProject/Blueprints/Player/Global/BP_EtherPlayerController.CheckVRMode` (`GameplayStatics.GetPlayerController` 0)))
    (if (not _result)
      (`SceneComponent.SetVisibility` _cube true false)
      (`SceneComponent.SetHiddenInGame` _cube false false)
      (`SceneComponent.SetVisibility` (`self.Widget`) true false)
      (`PrimitiveComponent.SetCollisionProfileName` (`self.BlockingVolume`) "BlockAllDynamic")
      (`PrimitiveComponent.SetCollisionProfileName` (`self.Cube`) "BlockAllDynamic"))))

(fn `UserConstructionScript`)