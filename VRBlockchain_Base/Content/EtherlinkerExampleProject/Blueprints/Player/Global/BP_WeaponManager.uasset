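; BP_WeaponManager declares weapon manager operations for the Etherlinker example project: initializing from a contract name and address, and creating weapons by name and type.
; Separate OnServerFromUI variants of both operations indicate requests passed from the UI to the server.
; A setter and getter pair is declared for the weapon manager menu widget.
; All functions are stubs with no logic, returning nothing or false.
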(fn `CreateNewWeapon`
  (params (Name :type String) (Type :type Integer))
  (return))

(fn `CreateNewWeaponOnServerFromUI`
  (params (Name :type String) (Type :type Integer))
  (return))

(fn `GetWeaponManagerMenuWidget`
  (returns (WeaponMangerMenuWidget :type "UserWidget Object Reference"))
  (return null))

(fn `InitializeWeaponManager`
  (params (ContractName :type String) (ContractAddress :type String))
  (returns (Result :type Boolean))
  (return false))

(fn `InitializeWeaponManagerOnServerFromUI`
  (params (ContractAddress :type String) (ContractName :type String))
  (returns (Result :type Boolean))
  (return false))

(fn `SetWeaponManagerMenuWidget`
  (params (WeaponMangerMenuWidget :type "UserWidget Object Reference"))
  (return))