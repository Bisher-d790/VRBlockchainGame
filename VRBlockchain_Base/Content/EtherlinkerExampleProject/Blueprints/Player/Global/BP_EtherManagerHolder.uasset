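; Blueprint interface for an Etherlinker player-side holder of the Ethereum manager, exposing wallet and response-handling functions without implementation.
; Covers creating, initializing, saving, loading and clearing local or remote wallets, with OnServerFromUI variants for widget requests.
; Wallet card functions pass a master password and encrypted wallet data between server and client through an authentication device.
; Also declares accessors for managers and authentication widgets, server travel, and EtherInteractor response callbacks.
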(fn `CheckWalletInitialization`
  (returns (Result :type Boolean))
  (return false))

(fn `ClearWalletData`
  (returns (Result :type Boolean))
  (return false))

(fn `ClearWalletDataOnServerFromUI`)

(fn `CreateLocalWallet`
  (params (Password :type String))
  (returns (Result :type Boolean))
  (return false))

(fn `CreateLocalWalletOnServerFromUI`
  (params (Password :type String) (ResultTextName :type String)))

(fn `CreateRemoteWallet`
  (params (Login :type String) (Password :type String))
  (returns (Result :type Boolean))
  (return false))

(fn `CreateRemoteWalletOnServerFromUI`
  (params (Login :type String) (Password :type String) (ResultTextName :type String)))

(fn `Execute On Batch Response Received`
  (params (EtherInteractor :type "ActorComponent Object Reference") (Result :type String) (Data :type "EtherlinkerBatchResponseData Structure"))
  (return))

(fn `Execute On Response Received`
  (params (EtherInteractor :type "ActorComponent Object Reference") (Result :type String) (Data :type "EtherlinkerResponseData Structure")))

(fn `Execute Update Bindings`
  (params (EtherInteractor :type "ActorComponent Object Reference")))

(fn `GetCurrentWalletData`
  (returns (WalletData :type "WalletData Structure"))
  (return))

(fn `GetEthereumManager`
  (returns (EtherManager :type "EtherManager Object Reference"))
  (return null))

(fn `GetEtherlinkerRemoteWalletManager`
  (returns (EtherlinkerRemoteWalletManager :type "EtherlinkerRemoteWalletManager Object Reference"))
  (return null))

(fn `GetUserIndex`
  (returns (UserIndex :type Integer))
  (return 0))

(fn `GetWalletAddress`
  (returns (WalletAddress :type String))
  (return ""))

(fn `GetWalletAuthenticationWidget`
  (returns (WalletAuthenticationWidget :type "UserWidget Object Reference"))
  (return null))

(fn `GetWalletCardMasterPassword`
  (returns (MasterPassword :type String))
  (return ""))

(fn `GetWalletCardMasterPasswordWidget`
  (returns (WalletCardMasterPasswordWidget :type "UserWidget Object Reference"))
  (return null))

(fn `InitializeRemoteWallet`
  (params (Login :type String) (Password :type String))
  (returns (Result :type Boolean))
  (return false))

(fn `InitializeRemoteWalletOnServerFromUI`
  (params (Login :type String) (Password :type String) (ResultTextName :type String)))

(fn `InitializeWallet`
  (params (WalletAddress :type String) (WalletPassword :type String) (WalletMnemonic :type String) (WalletPath :type String) (WalletAuthType :type String))
  (returns (Result :type Boolean))
  (return false))

(fn `InitializeWalletDataFromWalletCardOnServer`
  (params (IsWalletDataStored :type Boolean) (EncryptedWalletAddress :type String) (EncryptedWalletPassword :type String) (EncryptedWalletMnemonic :type String) (EncryptedWalletPath :type String) (EncryptedWalletAuthType :type String) (AuthenticationDevice :type "Actor Object Reference")))

(fn `InitializeWalletOnServerFromUI`
  (params (WalletAddress :type String) (WalletPassword :type String) (WalletMnemonic :type String) (WalletPath :type String) (WalletAuthType :type String) (ResultTextName :type String)))

(fn `LoadWalletFromFile`
  (params (Filename :type String) (Password :type String))
  (returns (Result :type Boolean))
  (return false))

(fn `LoadWalletFromFileOnServerFromUI`
  (params (Filename :type String) (Password :type String) (ResultTextName :type String)))

(fn `SaveWalletToFile`
  (params (Filename :type String) (Password :type String))
  (returns (Result :type Boolean))
  (return false))

(fn `SaveWalletToFileOnServerFromUI`
  (params (Filename :type String) (Password :type String) (ResultTextName :type String)))

(fn `ServerTravelFromUI`
  (params (Level :type String)))

(fn `SetWalletAuthenticationWidget`
  (params (WalletAuthenticationWidget :type "UserWidget Object Reference")))

(fn `SetWalletCardMasterPassword`
  (params (MasterPassword :type String))
  (returns (Result :type Boolean))
  (return false))

(fn `SetWalletCardMasterPasswordOnServerFromUI`
  (params (MasterPassword :type String)))

(fn `SetWalletCardMasterPasswordWidget`
  (params (WalletCardMasterPasswordWidget :type "UserWidget Object Reference")))

(fn `StoreWalletDataToWalletCardOnServer`
  (params (AuthenticationDevice :type "Actor Object Reference")))

(fn `UpdateWalletCardDataOnClient`
  (params (AuthenticationDevice :type "Actor Object Reference") (EncryptedWalletAddress :type String) (EncryptedWalletPassword :type String) (EncryptedWalletMnemonic :type String) (EncryptedWalletPath :type String) (EncryptedWalletAuthType :type String) (IsWalletDataStored :type Boolean)))

(fn `UpdateWalletCardInfoOnClient`
  (params (AuthenticationDevice :type "Actor Object Reference") (Result :type String) (WalletAddress :type String)))