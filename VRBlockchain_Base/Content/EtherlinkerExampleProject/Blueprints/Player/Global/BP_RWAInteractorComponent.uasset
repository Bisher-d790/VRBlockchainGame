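; BP_RWAInteractorComponent is a component from the Etherlinker example project that sends wallet data and account creation requests to an EtherlinkerRemoteWalletManager.
; On BeginPlay it messages every PlayerState to update bindings, retrying while the PlayerArray is empty.
; UpdateBindings, commented as server-side, binds its response handler to each PlayerState's wallet manager.
; Responses are rebroadcast through an event dispatcher when their UserIndex matches any PlayerState's index.
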(event `Execute`
  (params (EtherlinkerRemoteWalletManager :type "EtherlinkerRemoteWalletManager Object Reference") (RequestData :type "WalletAuthenticationRequest Structure") (OperationType :type "/Game/EtherlinkerExampleProject/Blueprints/Player/Global/BP_RWAOperationTypes Enum" :default "NewEnumerator0"))
  ;[1 1 1] Execute requested method
  (`/Engine/EditorBlueprintResources/StandardMacros.IsValid` EtherlinkerRemoteWalletManager
    (:`Is Valid`
      (switch `/Game/EtherlinkerExampleProject/Blueprints/Player/Global/BP_RWAOperationTypes` OperationType
        (:`NewEnumerator0`
          (`EtherlinkerRemoteWalletManager.GetWalletData` EtherlinkerRemoteWalletManager RequestData))
        (:`NewEnumerator1`
          (`EtherlinkerRemoteWalletManager.CreateUserAccount` EtherlinkerRemoteWalletManager RequestData))))))

(event `OnResponseReceived`
  (params (Result :type String) (Data :type "WalletAuthenticationResponse Structure"))
  (bind _playerarray (`GameStateBase.PlayerArray` (`GameplayStatics.GetGameState`)))
  ;[1 1 1] Call OnResponseReceived
  (if (> (`KismetArrayLibrary.Array_Length` _playerarray) 0)
    (for _array_element _playerarray
      (bind _userindex (message `/Game/EtherlinkerExampleProject/Blueprints/Player/Global/BP_EtherManagerHolder.GetUserIndex` _array_element))
      (if (== _userindex (`KismetStringLibrary.Conv_StringToInt` (`.userIndex` (break `WalletAuthenticationResponse` Data))))
        (`self.OnResponseReceivedEvent` Result Data)
        (break)))))

(event `self.ReceiveBeginPlay`
  (bind _playerarray (`GameStateBase.PlayerArray` (`GameplayStatics.GetGameState`)))
  ;[1 1 1] Bind OnResponseReceived event on server side from client
  ;;[0.1812 0.1812 0.1812] From Local to Server on all Player States
  (if (> (`KismetArrayLibrary.Array_Length` _playerarray) 0) :!label _label
    (for _array_element _playerarray
      (message `/Game/EtherlinkerExampleProject/Blueprints/Player/Global/BP_EtherManagerHolder.Execute Update Bindings` _array_element self))
    (else
      (`KismetSystemLibrary.Delay` 0.1)
      (goto _label))))

(event `/Game/EtherlinkerExampleProject/Blueprints/Player/Global/BP_EtherInteractor.UpdateBindings`
  (bind _playerarray (`GameStateBase.PlayerArray` (`GameplayStatics.GetGameState`)))
  ;[1 1 1] Bind OnResponseReceived event on server side from client
  ;;[0.1812 0.1812 0.1812] On Server for all Player States
  (if (> (`KismetArrayLibrary.Array_Length` _playerarray) 0) :!label _label_2
    (for _array_element _playerarray
      (bind _etherlinkerremotewalletmanager (message `/Game/EtherlinkerExampleProject/Blueprints/Player/Global/BP_EtherManagerHolder.GetEtherlinkerRemoteWalletManager` _array_element))
      (`/Engine/EditorBlueprintResources/StandardMacros.IsValid` _etherlinkerremotewalletmanager
        (:`Is Valid`
          (add `EtherlinkerRemoteWalletManager.OnResponseReceivedEvent` _etherlinkerremotewalletmanager (delegate `OnResponseReceived`)))))
    (else
      (`KismetSystemLibrary.Delay` 0.1)
      (goto _label_2))))