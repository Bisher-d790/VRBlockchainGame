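; BP_WeaponTokenmanager declares an interface-style API for managing weapon tokens in the Etherlinker example project, with no logic in any function body.
; It covers contract initialization, weapon creation, level-up, transfer, and detail and owner-index queries.
; Each operation pairs a boolean-returning function with an OnServerFromUI counterpart, named for server calls from menus.
; A setter and getter expose the token manager menu widget, passed in as an ERC721 admin menu.
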(fn `CreateNewWeapon`
  (params (Name :type String) (Type :type Integer))
  (returns (Result :type Boolean))
  (return false))

(fn `CreateNewWeaponOnServerFromUI`
  (params (Name :type String) (Type :type Integer)))

(fn `GetWeaponDetails`
  (params (WeaponID :type Integer))
  (returns (Result :type Boolean))
  (return false))

(fn `GetWeaponDetailsOnServerFromUI`
  (params (WeaponID :type Integer)))

(fn `GetWeaponsIndexes`
  (params (OwnerAddress :type String))
  (returns (Result :type Boolean))
  (return false))

(fn `GetWeaponsIndexesOnServerFromUI`
  (params (OwnerAddress :type String)))

(fn `GetWeaponTokenManagerMenuWidget`
  (returns (ERC721TokenAdminMenuWidget :type "UserWidget Object Reference"))
  (return null))

(fn `InitializeWeaponTokenManager`
  (params (ContractAddress :type String) (ContractName :type String))
  (returns (Result :type Boolean))
  (return false))

(fn `InitializeWeaponTokenManagerOnServerFromUI`
  (params (ContractAddress :type String) (ContractName :type String)))

(fn `LevelUpWeapon`
  (params (WeaponID :type Integer))
  (returns (Result :type Boolean))
  (return false))

(fn `LevelUpWeaponOnServerFromUI`
  (params (WeaponID :type Integer)))

(fn `SetWeaponTokenManagerMenuWidget`
  (params (ERC721TokenAdminMenuWidget :type "UserWidget Object Reference")))

(fn `TransferWeaponTo`
  (params (Owner :type String) (Target :type String) (WeaponID :type Integer))
  (returns (Result :type Boolean))
  (return false))

(fn `TransferWeaponToOnServerFromUI`
  (params (Owner :type String) (Target :type String) (WeaponID :type Integer)))