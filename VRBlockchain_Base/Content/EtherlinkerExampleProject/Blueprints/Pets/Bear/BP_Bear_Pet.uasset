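; Bear pet pawn that represents an ERC721 entity and follows its owning pawn.
; Initialize stores the token's name, DNA, owner wallet address, entity ID and owner pawn.
; PawnSensing sight and noise events trigger an AI move toward the owner only, stopping at an acceptance radius; a delayed follow chain is left unconnected.
; The Name RepNotify writes the name into the pet's wallet-card widget.
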(event `/Game/EtherlinkerExampleProject/Blueprints/Player/Global/BP_ERC721EntityActor.Initialize`
  (params (Name :type String) (DNA :type String) (OwnerWalletAddress :type String) (EntityID :type String) (OwnerPawn :type "Pawn Object Reference"))
  ;[1 1 1] Initialize ERC721 Entity
  (set `self.Name` Name)
  (set `self.DNA` DNA)
  (set `self.OwnerWalletAddress` OwnerWalletAddress)
  (set `self.EntityId` EntityID)
  (set `self.OwnerPawn` OwnerPawn))

(event `self.PawnSensing.OnSeePawn`
  (params (Pawn :type "Pawn Object Reference"))
  ;[1 1 1] Move to the owner
  (if (== (`self.OwnerPawn`) Pawn)
    (`|AIMoveTo` self (0.0 0.0 0.0) Pawn 400.0)))

(event `self.ReceiveTick`
  (params (DeltaSeconds :type "Float (single-precision)"))
  ;[1 1 1] Move to the owner
)

(event `self.PawnSensing.OnHearNoise`
  (params (Instigator :type "Pawn Object Reference") (Location :type "Vector Structure (by ref)") (Volume :type "Float (single-precision)"))
  ;[1 1 1] Move to the owner
  (if (== (`self.OwnerPawn`) Instigator)
    (`|AIMoveTo` self (0.0 0.0 0.0) Instigator 400.0)))

(fn `OnRep_Name`
  (`TextBlock.SetText` (`/Game/EtherlinkerExampleProject/Blueprints/UI/Widgets/BP_WalletCardAddress_UI.Terminal_Text` (cast `/Game/EtherlinkerExampleProject/Blueprints/UI/Widgets/BP_WalletCardAddress_UI` (`WidgetComponent.GetUserWidgetObject` (`self.Widget`)) :!pure true)) (`KismetTextLibrary.Conv_StringToText` (`self.Name`))))

(fn `UserConstructionScript`)